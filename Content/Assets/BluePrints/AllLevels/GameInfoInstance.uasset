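; Game instance that drives menu flow and multiplayer session handling.
; A save-slot check opens the main menu or, without a save, the options menu; most widgets are cached, while the server menu is recreated each time.
; It creates sessions and opens Lobby as a listen server, joins or destroys sessions, and shows a loading screen.
; Failures route to DisplayErrorMessage, which is empty, as are the strings from both error converters.
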(event Custom|ShowMainMenu
  (bind _returnvalue (Game|GetPlayerController 0))
  ;[1 1 1] 创建主菜单，显示鼠标
  (Utilities|IsValid (Variables|Widgets|GetMainMenuWB)
    (:Is%20Valid
      _)
    (:Is%20Not%20Valid
      (bind _returnvalue_2 (UserInterface|CreateWidget "/Game/Assets/UI/MainMenu/MainMenu.MainMenu_C" _returnvalue))
      (Variables|Widgets|SetMainMenuWB _returnvalue_2)))
  (UserInterface|Viewport|AddtoViewport (Variables|Widgets|GetMainMenuWB) 0)
  (Variables|/Script/Engine.PlayerController|SetbShowMouseCursor _returnvalue true))

(event Custom|ShowHostMenu
  ;[1 1 1] 显示主菜单
  (Utilities|IsValid (Variables|Widgets|GetHostMenuWB)
    (:Is%20Valid
      _)
    (:Is%20Not%20Valid
      (bind _returnvalue (UserInterface|CreateWidget "/Game/Assets/UI/MainMenu/HostMenu.HostMenu_C" (Game|GetPlayerController 0)))
      (Variables|Widgets|SetHostMenuWB _returnvalue)))
  (UserInterface|Viewport|AddtoViewport (Variables|Widgets|GetHostMenuWB) 0))

(event Custom|ShowServerMenu
  ;[1 1 1] 显示服务器菜单，每次显示都是新的
  (bind _returnvalue (UserInterface|CreateWidget "/Game/Assets/UI/MainMenu/ServerMenu.ServerMenu_C" (Game|GetPlayerController 0)))
  (UserInterface|Viewport|AddtoViewport _returnvalue 0))

(event Custom|ShowOptionMenu
  ;[1 1 1] 显示选项菜单
  (Utilities|IsValid (Variables|Widgets|GetOptionMenuWB)
    (:Is%20Valid
      _)
    (:Is%20Not%20Valid
      (bind _returnvalue (UserInterface|CreateWidget "/Game/Assets/UI/MainMenu/OptionMenu.OptionMenu_C" (Game|GetPlayerController 0)))
      (Variables|Widgets|SetOptionMenuWB _returnvalue)))
  (UserInterface|Viewport|AddtoViewport (Variables|Widgets|GetOptionMenuWB) 0))

(event Custom|LaunchLobby
  (params (NumberOfPlayers :type Integer) (EnableLAN :type Boolean) (ServerName :type Text))
  ;[1 1 1] LaunchLobby打开带有主机设置的大厅
  (Variables|ServerSettings|SetMaxPlayers NumberOfPlayers) ; Replicated
  (Variables|ServerSettings|SetServerName ServerName) ; Replicated
  (CallFunction|ShowLoadingScreen)
  (|Session (Game|GetPlayerController 0) (Variables|ServerSettings|GetMaxPlayers) EnableLAN
    (:OnSuccess
      (Game|OpenLevel(byName) "Lobby" true "listen"))
    (:OnFailure
      (Utilities|DisplayErrorMessage "Faild to Session. Please Try Again."))))

(event Custom|ShowLoadingScreen
  ;[1 1 1] 显示要加载加载中的屏幕
  (Utilities|IsValid (Variables|Default|GetLoadingScreenWB)
    (:Is%20Valid
      _)
    (:Is%20Not%20Valid
      (bind _returnvalue (UserInterface|CreateWidget "/Game/Assets/UI/AllLevels/LoadingScreen.LoadingScreen_C" (Game|GetPlayerController 0)))
      (Variables|Default|SetLoadingScreenWB _returnvalue)))
  (UserInterface|Viewport|AddtoViewport (Variables|Default|GetLoadingScreenWB) 0))

(event Custom|JoinServer
  (params (SessionToJoin :type Blueprint%20Session%20Result%20Structure))
  ;[1 1 1] 加入服务器，导入服务器菜单
  (CallFunction|ShowLoadingScreen)
  (|JoinSession (Game|GetPlayerController 0) SessionToJoin
    (:OnFailure
      (Utilities|DisplayErrorMessage "Faild to Join Session. Please Try Again."))))

(event Custom|DestroySessionCollor
  (params (PlayerController :type Player%20Controller%20Object%20Reference))
  ;[1 1 1] 销毁会话，退出服务器
  (|DestroySession PlayerController))

(event Custom|SaveGameCheck
  ;[1 1 1] 检查保存文件（检查存档）
  (bind _returnvalue (SaveGame|DoesSaveGameExist (Variables|Default|GetPlayerSettingSave))) ; 查询游戏存档在不在
  (if _returnvalue
    (CallFunction|ShowMainMenu)
    (Variables|Default|SetCreateSaveFile? true)
    (else
      (CallFunction|ShowOptionMenu)
      (Variables|/Script/Engine.PlayerController|SetbShowMouseCursor (Game|GetPlayerController 0) true))))

(event EventHandleNetworkError
  (params (FailureType :type ENetworkFailure%20Enum :default "NetDriverAlreadyExists") (bIsServer :type Boolean))
  ;[1 1 1] 网络错误处理和消息输出
  (if bIsServer
    _
    (else
      _))
  (Utilities|DisplayErrorMessage (CallFunction|NetErrortoString FailureType)))

(event EventHandleTravelError
  (params (FailureType :type ETravelFailure%20Enum :default "NoLevel"))
  ;[1 1 1] 漫游错误处理和消息输出
  (Utilities|DisplayErrorMessage (CallFunction|TravelErrortoString FailureType)))

(fn NetErrortoString
  (params (FailureType :type ENetworkFailure%20Enum :default "NetDriverAlreadyExists"))
  (return ""))

(fn TravelErrortoString
  (params (FailureType :type ETravelFailure%20Enum :default "NoLevel"))
  (return ""))