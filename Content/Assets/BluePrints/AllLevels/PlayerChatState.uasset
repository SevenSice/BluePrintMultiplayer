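; PlayerChatState relays lobby chat messages, prefixed with the sender's name.
; On BeginPlay it takes that name from the player settings of player controller 0, cast to Loby_PC.
; Server-SandMessage formats name and text, then calls All-SandMessage, following a server-to-all naming pattern.
; All-SandMessage finds the first LobbyMenu widget and passes the line to its ChatWindow.
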(event Custom|Server-SandMessage
  (params (Message :type Text))
  (CallFunction|All-SandMessage (Utilities|Text|FormatText "{Name}：{Message}" (Variables|Default|GetNameOfSender) Message)))

(event Custom|All-SandMessage
  (params (Message :type Text))
  (bind _foundwidgets (Widget|GetAllWidgetsOfClass "/Game/Assets/UI/Lobby/LobbyMenu.LobbyMenu_C" false))
  (Default|OnMessageReceived (Variables|/Game/Assets/UI/Lobby/LobbyMenu.LobbyMenu_C|GetChatWindow (Utilities|Array|Get(acopy) _foundwidgets)) Message))

(event EventBeginPlay
  (bind _asloby_pc (Utilities|Casting|CastToLoby_PC (Game|GetPlayerController 0)))
  (Variables|Default|SetNameOfSender (.MyplayerName (Utilities|Struct|BreakPlayerInfo (Variables|/Game/Assets/BluePrints/Lobby/Loby_PC.Loby_PC_C|GetPlayerSettings _asloby_pc)))))

(fn ConstructionScript)