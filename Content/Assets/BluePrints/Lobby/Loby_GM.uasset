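; Lobby game mode that tracks joining players, map settings and start readiness, then server-travels to the selected arena.
; On post-login it sets up each Loby_PC from the game instance's server settings and possesses a placeholder 0_Base pawn at a random PlayerStart.
; EveryOneUpdate pushes player info and available characters to all controllers, blocking start readiness while a player keeps the placeholder character.
; Map changes are relayed to every controller; SwapCharacter is an empty stub.
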(event Custom|SwapCharacter
  (params (PlayerController :type Player%20Controller%20Object%20Reference) (CharacterClass :type Character%20Class%20Reference) (ChangedStatus :type Boolean)))

(event Custom|EveryOneUpdate
  (bind _allplayercontrollers (Variables|ServerSettings|GetAllPlayerControllers))
  ;[1 1 1] 广播大厅更新给大厅玩家（呼叫时将大厅更新信息传给呼叫者）
  (bind _output_get (Variables|ServerSettings|SetCurrentPlayers (Utilities|Array|Length (Variables|ServerSettings|GetAllPlayerControllers))))
  (if (> _output_get 0)
    (Utilities|Array|Clear (Variables|ServerSettings|GetConnectedPlayers))
    (for _array_element _allplayercontrollers
      (bind _asloby_pc (Utilities|Casting|CastToLoby_PC _array_element))
      (Utilities|Array|Add (Variables|ServerSettings|GetConnectedPlayers) (Variables|/Game/Assets/BluePrints/Lobby/Loby_PC.Loby_PC_C|GetPlayerSettings _asloby_pc))
      (Default|UpdateNumberOfPlayers _asloby_pc (Variables|ServerSettings|GetCurrentPlayers) (Variables|ServerSettings|GetMaxPlayers)))
    (for _array_element_2 _allplayercontrollers
      (bind _asloby_pc_2 (Utilities|Casting|CastToLoby_PC _array_element_2))
      (Default|AddPlayerInfo _asloby_pc_2 (Variables|ServerSettings|GetConnectedPlayers))
      (Default|UpdateAvailableCharacter _asloby_pc_2 (Variables|ServerSettings|GetAvailableCharacrters))
      (CallFunction|AddtoTackList))
    (bind _array_element_3 (Utilities|Array|ForEachLoopwithBreak (Variables|ServerSettings|GetConnectedPlayers))
      (:LoopBody
        (if (== (.MyPlayerCharactor (Utilities|Struct|BreakPlayerInfo _array_element_3)) "/Game/Assets/BluePrints/Charactors/0_Base.0_Base_C")
          (Variables|ServerSettings|SetCanWeStart? false)
          (CallFunction|CannotStartGame)
          (else
            (Variables|ServerSettings|SetCanWeStart? true)))))))

(event Custom|LaunchTheGame
  (switch int (Variables|ServerSettings|GetGM_MapID)
    (:Default
      (Development|ExecuteConsoleCommand "servertravel /Game/Assets/Maps/Arena01" 0 :!label _label))
    (:0
      (goto _label))
    (:1
      (Development|ExecuteConsoleCommand "servertravel /Game/Assets/Maps/Arena02" 0))))

(event Custom|ReSpawnPlayer
  (params (PlayerController :type Player%20Controller%20Object%20Reference))
  (bind _returnvalue (Pawn|GetControlledPawn PlayerController))
  (bind _spawnpoint (Variables|ServerSettings|GetSpawnPoint))
  ;[1 1 1] 进入大厅时，创建基本角色。通知其它玩家更新大厅信息
  (Utilities|IsValid _returnvalue
    (:Is%20Valid
      (Actor|DestroyActor _returnvalue))
    (:Is%20Not%20Valid
      _))
  (bind _returnvalue_2 (Game|SpawnActorfromClass "/Game/Assets/BluePrints/Charactors/0_Base.0_Base_C" (Transformation|GetActorTransform (Utilities|Array|Get(acopy) _spawnpoint (Math|Random|RandomIntegerinRange 0 (- (Utilities|Array|Length _spawnpoint) 1)))) "Undefined" 0 0))
  (Pawn|Possess PlayerController _returnvalue_2)
  (CallFunction|EveryOneUpdate))

(event Custom|AddToTackList)

(event Custom|CannotStartGame
  ;[1 1 1] 广播大厅更新给大厅玩家（呼叫时将大厅更新信息传给呼叫者）
  (Utilities|Array|ForEachLoopwithBreak (Variables|ServerSettings|GetConnectedPlayers)) ; enters at Break
)

(event Custom|ServerUpdateGameSettings
  (params (MapImage :type Texture%202D%20Object%20Reference) (MapName :type Text) (MapTime :type Text) (MapID :type Integer))
  ;[1 1 1] 如果服务器有更新，通知各个客户端更新大厅信息
  (Variables|ServerSettings|SetGM_MapImage MapImage)
  (Variables|ServerSettings|SetGM_MapName MapName)
  (Variables|ServerSettings|SetGM_MapTime MapTime)
  (Variables|ServerSettings|SetGM_MapID MapID)
  (for _array_element (Variables|ServerSettings|GetAllPlayerControllers)
    (bind _asloby_pc (Utilities|Casting|CastToLoby_PC _array_element))
    (Default|UpdateLobbySettings _asloby_pc (Variables|ServerSettings|GetGM_MapImage) (Variables|ServerSettings|GetGM_MapName) (Variables|ServerSettings|GetGM_MapTime))))

(event EventPostLogin
  (params (NewPlayer :type Player%20Controller%20Object%20Reference))
  ;[1 1 1] 登陆后初始化，配置玩家控制器信息和在玩家客户端上创建角色
  (Networking|SwitchHasAuthority
    (:Authority
      (Utilities|Array|Add (Variables|ServerSettings|GetAllPlayerControllers) NewPlayer)
      (bind _outactors (Actor|GetAllActorsOfClass "/Script/Engine.PlayerStart"))
      (Variables|ServerSettings|SetSpawnPoint _outactors)
      (bind _asgame_info_instance (Utilities|Casting|CastToGameInfoInstance (Game|GetGameInstance)))
      (Variables|ServerSettings|SetServerName (Variables|/Game/Assets/BluePrints/AllLevels/GameInfoInstance.GameInfoInstance_C|GetServerName _asgame_info_instance))
      (Variables|ServerSettings|SetMaxPlayers (Variables|/Game/Assets/BluePrints/AllLevels/GameInfoInstance.GameInfoInstance_C|GetMaxPlayers _asgame_info_instance))
      (bind _asloby_pc (Utilities|Casting|CastToLoby_PC NewPlayer))
      (Default|InitialSetup _asloby_pc)
      (Default|SetupLobbyMenu _asloby_pc (Variables|ServerSettings|GetServerName))
      (Default|UpdateLobbySettings _asloby_pc (Variables|ServerSettings|GetGM_MapImage) (Variables|ServerSettings|GetGM_MapName) (Variables|ServerSettings|GetGM_MapTime))
      (CallFunction|ReSpawnPlayer NewPlayer))))

(fn ConstructionScript)